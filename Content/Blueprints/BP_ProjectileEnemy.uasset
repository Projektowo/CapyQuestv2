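; BP_ProjectileEnemy is a projectile, by its name fired by enemies, that damages BP_Character actors.
; The construction script feeds its speed and velocity variables into ProjectileMovement.
; Overlapping a BP_Character calls Hit, which applies damage to every overlapping BP_Character, then destroys the projectile.
; A blocking hit on the sphere destroys it without damage, and a short timed lifetime also removes it.
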(event `self.ReceiveBeginPlay`
  (`KismetSystemLibrary.Delay` 3.0)
  (`self.K2_DestroyActor`))

(event `self.Sphere.OnComponentBeginOverlap`
  (params (OverlappedComponent :type "PrimitiveComponent Object Reference") (OtherActor :type "Actor Object Reference") (OtherComp :type "PrimitiveComponent Object Reference") (OtherBodyIndex :type Integer) (bFromSweep :type Boolean) (SweepResult :type "HitResult Structure (by ref)"))
  (cast `/Game/Blueprints/BP_Character` OtherActor)
  (`self.Hit`)
  (`self.K2_DestroyActor`))

(event `self.Sphere.OnComponentHit`
  (params (HitComponent :type "PrimitiveComponent Object Reference") (OtherActor :type "Actor Object Reference") (OtherComp :type "PrimitiveComponent Object Reference") (NormalImpulse :type "Vector Structure") (Hit :type "HitResult Structure (by ref)"))
  (`self.K2_DestroyActor`))

(fn `Hit`
  (for _array_element (`PrimitiveComponent.GetOverlappingActors` (`self.Sphere`) "/Game/Blueprints/BP_Character.BP_Character_C")
    (if (!= _array_element self)
      (`GameplayStatics.ApplyDamage` _array_element (`self.Damage`)))))

(fn `UserConstructionScript`
  (bind _projectilemovement (`self.ProjectileMovement`))
  (bind _projectilespeed (`self.ProjectileSpeed`))
  (set `ProjectileMovementComponent.MaxSpeed` _projectilespeed _projectilemovement)
  (set `ProjectileMovementComponent.InitialSpeed` _projectilespeed _projectilemovement)
  (set `MovementComponent.Velocity` (`self.ProjectileVelocity`) _projectilemovement))