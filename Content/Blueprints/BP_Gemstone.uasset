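; BP_Gemstone is a collectible gem pickup that adds to the player character's score.
; On BeginPlay it sets its Paper2D sprite to a random pick from eight gem sprites, so the look varies per instance.
; When a BP_Character overlaps its sphere, it adds Amount, truncated to an integer, to that character's Score and destroys itself.
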(event `self.Sphere.OnComponentBeginOverlap`
  (params (OverlappedComponent :type "PrimitiveComponent Object Reference") (OtherActor :type "Actor Object Reference") (OtherComp :type "PrimitiveComponent Object Reference") (OtherBodyIndex :type Integer) (bFromSweep :type Boolean) (SweepResult :type "HitResult Structure (by ref)"))
  (bind _asbp_character (cast `/Game/Blueprints/BP_Character` OtherActor))
  (set `/Game/Blueprints/BP_Character.Score` (`KismetMathLibrary.FTrunc` (+ (`/Game/Blueprints/BP_Character.Score` _asbp_character) (`self.Amount`))) _asbp_character)
  (`self.K2_DestroyActor`))

(event `self.ReceiveBeginPlay`
  (`PaperSpriteComponent.SetSprite` (`self.PaperSprite`) (`KismetArrayLibrary.Array_Random` (`|MakeArray` "/Game/Sprites/gemstones/amethyst_Sprite_0.amethyst_Sprite_0" "/Game/Sprites/gemstones/citrine_Sprite_0.citrine_Sprite_0" "/Game/Sprites/gemstones/diamond_Sprite_0.diamond_Sprite_0" "/Game/Sprites/gemstones/emerald_Sprite_0.emerald_Sprite_0" "/Game/Sprites/gemstones/love_Sprite_0.love_Sprite_0" "/Game/Sprites/gemstones/ruby_Sprite_0.ruby_Sprite_0" "/Game/Sprites/gemstones/zirconia_Sprite_0.zirconia_Sprite_0" "/Game/Sprites/gemstones/topaz_Sprite_0.topaz_Sprite_0" :!type "PaperSprite Object Reference"))))

(fn `UserConstructionScript`)