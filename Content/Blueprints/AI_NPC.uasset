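; AI controller for NPCs that runs the BT_NPC behavior tree and feeds it AI Perception results through the Blackboard.
; Touch and sight set or clear the player as TargetActor; losing sight also stores LastKnownLocation.
; Hearing writes the sound's location to TargetLocation from any source.
; Each perception update also calls a turn-toward-player function, whose graph here holds only disconnected fixed-yaw rotation logic.
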(event OnTargetPerceptionUpdated(AIPerception)
  (params (Actor :type Actor%20Object%20Reference) (Stimulus :type AI%20Stimulus%20Structure))
  ;[1 1 1] Jezeli do przeciwnika cos dotrze, to odpali te eventy
  (Utilities|FlowControl|Sequence
    (:then_0
      (CallFunction|HandleTouchEvent Actor Stimulus)
      (|Obrótwkierunkugracza Actor))
    (:then_1
      (CallFunction|HandleSightSense Actor Stimulus)
      (CallFunction|HandleSoundSense Stimulus))))

(event EventBeginPlay
  ;[1 1 1] Inicjowanie drzewa AI
  (AI|RunBehaviorTree "/Game/Blueprints/BT_NPC.BT_NPC"))

(fn ConstructionScript)

(fn HandleSightSense
  (params (Actor :type Actor%20Object%20Reference) (Stimulus :type AI%20Stimulus%20Structure))
  ;[1 1 1] Jezeli zmysl wzroku
  (bind _returnvalue (Class|AIPerceptionSystem|GetSenseClassforStimulus Stimulus))
  (if (== _returnvalue "/Script/AIModule.AISense_Sight")
    (if (== Actor (Game|GetPlayerCharacter 0))
      ;[1 1 1] Wrzucenie do blackboarda gracza jako 'TargetActor
      (AI|Components|Blackboard|SetValueasObject (Variables|Default|GetBlackboard) (Utilities|Name|MakeLiteralName "TargetActor") (Utilities|SelectObject (Game|GetPlayerCharacter 0) 0 (.bsuccessfullysensed Stimulus)))
      ;[1 1 1] Jak przeciwnik stracił gracza z oczu, to dodaje do blackboarda wektor pod zmienną LastKnownLocation
      (if (not (.bsuccessfullysensed Stimulus))
        (AI|Components|Blackboard|SetValueasVector (Variables|Default|GetBlackboard) (Utilities|Name|MakeLiteralName "LastKnownLocation") (.stimuluslocation Stimulus)))
      (else
        (return)))
    (else
      (return))))

(fn HandleSoundSense
  (params (Stimulus :type AI%20Stimulus%20Structure%20%28by%20ref%29))
  ;[1 1 1] Czy zmysł słuchu
  (bind _returnvalue (Class|AIPerceptionSystem|GetSenseClassforStimulus Stimulus))
  ;[1 1 1] Przypisanie lokalizacji dzwieku w blackboardzie pod zmienna TargetLocation
  (if (== _returnvalue "/Script/AIModule.AISense_Hearing")
    (AI|Components|Blackboard|SetValueasVector (Variables|Default|GetBlackboard) (Utilities|Name|MakeLiteralName "TargetLocation") (.StimulusLocation (Utilities|Struct|BreakAIStimulus Stimulus)))))

(fn HandleTouchEvent
  (params (Actor :type Actor%20Object%20Reference) (Stimulus :type AI%20Stimulus%20Structure))
  ;[1 1 1] Czy dotyk
  (bind _returnvalue (Class|AIPerceptionSystem|GetSenseClassforStimulus Stimulus))
  (if (== _returnvalue "/Script/AIModule.AISense_Touch")
    ;[1 1 1] Ustawienie w blackboardzie gracza jako TargetActor
    (if (== Actor (Game|GetPlayerCharacter 0))
      (AI|Components|Blackboard|SetValueasObject (Variables|Default|GetBlackboard) (Utilities|Name|MakeLiteralName "TargetActor") (Utilities|SelectObject (Game|GetPlayerCharacter 0) 0 (.bsuccessfullysensed Stimulus)))
      (else
        (return)))
    (else
      (return))))