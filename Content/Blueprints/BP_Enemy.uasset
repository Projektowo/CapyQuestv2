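; Paper2D enemy Blueprint with health, a flipbook-timed melee attack and an AI Perception component.
; While attacking, Tick fires a DoOnce at sprite frame 3 to damage characters overlapping the hitbox, and ResetAttack re-arms it.
; Hit events report touch stimuli to the enemy itself.
; The perception update handler is empty, and the sight logic that writes blackboard targets is disconnected.
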(event `ResetAttack`
  ;[1 1 1] Attack sequence
  (goto _label :!via `Reset`))

(event `self.ReceiveTick`
  (params (DeltaSeconds :type "Float (single-precision)"))
  ;[1 1 1] Attack sequence
  (if (`self.IsAttacking?`)
    (if (== (`PaperFlipbookComponent.GetPlaybackPositionInFrames` (`self.Sprite`)) 3)
      (`/Engine/EditorBlueprintResources/StandardMacros.DoOnce` false :!label _label
        (:`Completed`
          (`self.HitCheck`))))))

(event `self.AIPerception.OnTargetPerceptionUpdated`
  (params (Actor :type "Actor Object Reference") (Stimulus :type "AIStimulus Structure")))

(event `self.ReceiveHit`
  (params (MyComp :type "PrimitiveComponent Object Reference") (Other :type "Actor Object Reference") (OtherComp :type "PrimitiveComponent Object Reference") (bSelfMoved :type Boolean) (HitLocation :type "Vector Structure") (HitNormal :type "Vector Structure") (NormalImpulse :type "Vector Structure") (Hit :type "HitResult Structure (by ref)"))
  ;[1 1 1] Zmysł dotyku
  (`AISense_Touch.ReportTouchEvent` self Other HitLocation))

(event `/Game/Blueprints/INT_EnemyStats.Stats`
  (params (Health :type Integer) (AttackRange :type "Float (double-precision)"))
  (set `self.Health` Health)
  (set `self.AttackRange` AttackRange))

(fn `HandleSightSense`
  (params (Actor :type "Actor Object Reference") (Stimulus :type "AIStimulus Structure")))

(fn `HitCheck`
  (for _array_element (`PrimitiveComponent.GetOverlappingActors` (`self.Hitbox`) "/Game/Blueprints/BP_Character.BP_Character_C")
    (if (!= _array_element self)
      (`GameplayStatics.ApplyDamage` _array_element (`self.Damage`)))))

(fn `RestartAnimation`
  (if (not (`PaperFlipbookComponent.IsPlaying` (`self.Sprite`)))
    (`PaperFlipbookComponent.Play` (`self.Sprite`))))

(fn `UserConstructionScript`
  (set `self.Health` (`self.DefaultHealth`)))