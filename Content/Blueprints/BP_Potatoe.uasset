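; BP_Potatoe is a potato enemy that supplies its own punch animation and stats on top of inherited enemy logic.
; MeleeAttackv3 plays the punch flipbook once and flags it as attacking; when the flipbook finishes, the sprite returns to looping idle, the attack resets and animation restarts.
; The construction script calls the parent, then sets this enemy's health and damage.
; Hitbox visibility toggles are present but never run.
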(event `self.MeleeAttackv3`
  ;[1 1 1] Potatoe attack
  (`PaperFlipbookComponent.SetFlipbook` (`self.Sprite`) "/Game/Sprites/enemy/Potatoe/Enemy_Potatoe/Enemy_Potatoe_Punch.Enemy_Potatoe_Punch")
  (`PaperFlipbookComponent.SetLooping` (`self.Sprite`) false)
  (set `self.IsAttacking?` true))

(event `self.Sprite.OnFinishedPlaying`
  ;[1 1 1] Potatoe attack
  (`PaperFlipbookComponent.SetFlipbook` (`self.Sprite`) "/Game/Sprites/enemy/Potatoe/Enemy_Potatoe/Enemy_Potatoe_Idle.Enemy_Potatoe_Idle")
  (`PaperFlipbookComponent.SetLooping` (`self.Sprite`) true)
  (`self.ResetAttack`)
  (set `self.IsAttacking?` false)
  (`self.RestartAnimation`))

(fn `UserConstructionScript`
  (`parent.UserConstructionScript`)
  (set `self.Health` 4)
  (set `self.Damage` 66.0))