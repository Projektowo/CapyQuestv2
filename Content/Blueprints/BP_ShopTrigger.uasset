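; Shop trigger actor that opens and closes the WB_Shop screen as actors enter and leave its ShopTrigger volume.
; Begin overlap requires INT_ShopInterface, creates a widget, and, if none is visible, shows it with a sound and mouse cursor.
; End overlap reverses this for any actor, without an interface check.
; BeginPlay caches the player's BP_Character, unused here, and both sounds play at world origin.
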(event `self.ReceiveBeginPlay`
  (`self.Casting`))

(event `self.ShopTrigger.OnComponentBeginOverlap`
  (params (OverlappedComponent :type "PrimitiveComponent Object Reference") (OtherActor :type "Actor Object Reference") (OtherComp :type "PrimitiveComponent Object Reference") (OtherBodyIndex :type Integer) (bFromSweep :type Boolean) (SweepResult :type "HitResult Structure (by ref)"))
  (if (`KismetSystemLibrary.DoesImplementInterface` OtherActor "/Game/Blueprints/INT_ShopInterface.INT_ShopInterface_C")
    (bind _returnvalue (`|CreateWidget` "/Game/Blueprints/Widgets/WB_Shop.WB_Shop_C" (`GameplayStatics.GetPlayerController` 0)))
    (if (not (`self.IsShopVisible?`))
      (`GameplayStatics.PlaySoundAtLocation` "/Game/Sounds/Shop/OpenShop.OpenShop" (0.0 0.0 0.0) (struct) 1.0 1.0 0.0 null null null null)
      (bind _output_get (set `self.ShopWidget` _returnvalue))
      (set `self.IsShopVisible?` true)
      (`UserWidget.AddToViewport` _output_get 0)
      (set `PlayerController.bShowMouseCursor` true (`GameplayStatics.GetPlayerController` 0)))))

(event `self.ShopTrigger.OnComponentEndOverlap`
  (params (OverlappedComponent :type "PrimitiveComponent Object Reference") (OtherActor :type "Actor Object Reference") (OtherComp :type "PrimitiveComponent Object Reference") (OtherBodyIndex :type Integer))
  (`Widget.RemoveFromParent` (`self.ShopWidget`))
  (`GameplayStatics.PlaySoundAtLocation` "/Game/Sounds/Shop/CloseShop.CloseShop" (0.0 0.0 0.0) (struct) 1.0 1.0 0.0 null null null null)
  (set `self.IsShopVisible?` false)
  (set `PlayerController.bShowMouseCursor` false (`GameplayStatics.GetPlayerController` 0)))

(fn `Casting`
  (bind _asbp_character (cast `/Game/Blueprints/BP_Character` (`GameplayStatics.GetPlayerPawn` 0)))
  (set `self.BP Character` _asbp_character))

(fn `UserConstructionScript`)