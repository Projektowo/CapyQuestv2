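; Patrol path point for AI that turns an arriving patroller to face the direction of its Arrow component.
; OnPatrollerEntered waits one second, then sets the character's controller rotation to the arrow's world rotation.
; An older gated Tick path for rotating the actor directly remains, marked as a relic; OnPatrollerExit closes its gate, but the logic that opens it is disconnected.
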(event `self.ReceiveActorBeginOverlap`
  (params (OtherActor :type "Actor Object Reference")))

(event `self.ReceiveTick`
  (params (DeltaSeconds :type "Float (single-precision)"))
  (bind _character (`self.Character`))
  ;[1 1 1] Kolejny relikt przeszlosci, bo wystarczylo kliknac jeden pierdolozuldfgvfzldsfb checkbox xDDDDDDDDDDDDDDD
  (`/Engine/EditorBlueprintResources/StandardMacros.Gate` true :!label _label
    (:`Exit`
      (`KismetSystemLibrary.Delay` 1.0)
      (`self.K2_SetActorRotation` _character (`KismetMathLibrary.RInterpTo` (`self.K2_GetActorRotation` _character) (`SceneComponent.K2_GetComponentRotation` (`self.Arrow`)) DeltaSeconds) false))))

(event `OnPatrollerExit`
  ;[1 1 1] Kolejny relikt przeszlosci, bo wystarczylo kliknac jeden pierdolozuldfgvfzldsfb checkbox xDDDDDDDDDDDDDDD
  (goto _label :!via `Close`))

(event `OnPatrollerEntered`
  (params (Character :type "Character Object Reference"))
  ;[1 1 1] Obraca postac w kierunku strzałki
  (`KismetSystemLibrary.Delay` 1.0)
  (`Controller.SetControlRotation` (`Pawn.GetController` Character) (`SceneComponent.K2_GetComponentRotation` (`self.Arrow`))))

(fn `UserConstructionScript`)