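; BP_Puma is a Paper2D puma character with a melee attack, driven by flipbook swaps on its sprite.
; MeleeAttackv3 plays the attack flipbook once and sets IsAttacking; when playback finishes, it returns to looping idle and resets the attack.
; The construction script sets Health and Damage.
; AnyDamage is empty: the hurt, death and hitbox visibility logic is disconnected and never runs.
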(event `self.MeleeAttackv3`
  ;[1 1 1] Puma
  (`PaperFlipbookComponent.SetFlipbook` (`self.Sprite`) "/Game/Sprites/enemy/Puma/attack/PumaAttack.PumaAttack")
  (`PaperFlipbookComponent.SetLooping` (`self.Sprite`) false)
  (set `self.IsAttacking?` true))

(event `self.Sprite.OnFinishedPlaying`
  ;[1 1 1] Puma
  (`PaperFlipbookComponent.SetFlipbook` (`self.Sprite`) "/Game/Sprites/enemy/Puma/idle/PumaIdle.PumaIdle")
  (`PaperFlipbookComponent.SetLooping` (`self.Sprite`) true)
  (`self.ResetAttack`)
  (set `self.IsAttacking?` false)
  (`self.RestartAnimation`))

(event `self.ReceiveAnyDamage`
  (params (Damage :type "Float (single-precision)") (DamageType :type "DamageType Object Reference") (InstigatedBy :type "Controller Object Reference") (DamageCauser :type "Actor Object Reference"))
  ;[1 1 1] Puma
  ;;[1 1 1] Getting damage and death
)

(fn `UserConstructionScript`
  (`parent.UserConstructionScript`)
  (set `self.Health` 3)
  (set `self.Damage` 33.0))