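; Behavior tree task that walks an AI pawn along the patrol path stored on its BP_AIBehaviourComponent.
; It moves to each point in the path map's key order, notifies it on arrival, waits for that point's mapped duration, then notifies exit and advances.
; At the path's end it either loops to the start or reverses direction, per the component's outcome setting.
; It only finishes, as failed, on missing data or a failed move.
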(event `self.ReceiveExecuteAI`
  (params (OwnerController :type "AIController Object Reference") (ControlledPawn :type "Pawn Object Reference"))
  (bind _returnvalue (`Actor.GetComponentByClass` ControlledPawn "/Game/Blueprints/BP_AIBehaviourComponent.BP_AIBehaviourComponent_C"))
  (bind _patrolpath (`/Game/Blueprints/BP_AIBehaviourComponent.PatrolPath` _returnvalue))
  (set `self.Controlled Pawn` ControlledPawn)
  (`/Engine/EditorBlueprintResources/StandardMacros.IsValid` _returnvalue
    (:`Is Valid`
      (set `self.Patrol Path Outcome` (`/Game/Blueprints/BP_AIBehaviourComponent.PatrolPathOutcome` _returnvalue))
      (if (> (`BlueprintMapLibrary.Map_Length` _patrolpath) 0)
        (set `self.PatrolPath` _patrolpath)
        (`self.MoveToPatrolPoint`)
        (else
          (`self.FinishExecute` false))))
    (:`Is Not Valid`
      (`self.FinishExecute` false))))

(event `MoveToPatrolPoint`
  (bind _patrolpath (`self.PatrolPath`))
  (bind _keys (`BlueprintMapLibrary.Map_Keys` (`self.PatrolPath`)))
  (`|AIMoveTo` (`self.Controlled Pawn`) (`Actor.K2_GetActorLocation` (`|GetArrayItem` _keys (`self.CurrentPatrolIndex`))) null
    (:`OnSuccess`
      (bind _keys_2 (`BlueprintMapLibrary.Map_Keys` _patrolpath))
      (bind _output (`|GetArrayItem` _keys_2 (`self.CurrentPatrolIndex`)))
      (set `self.CurrentPatrolPoint` _output)
      (`KismetSystemLibrary.K2_SetTimerDelegate` (delegate `OnEndWaiting`) (`KismetMathLibrary.FMax` (`BlueprintMapLibrary.Map_Find` _patrolpath _output) 0.1))
      (`/Game/Blueprints/BP_AIObject_PatrolPathpoint.OnPatrollerEntered` (`self.CurrentPatrolPoint`) (cast `Character` (`self.Controlled Pawn`) :!pure true)))
    (:`OnFail`
      (`self.FinishExecute` false))))

(event `OnEndWaiting`
  (`/Game/Blueprints/BP_AIObject_PatrolPathpoint.OnPatrollerExit` (`self.CurrentPatrolPoint`))
  (bind _output_get (set `self.CurrentPatrolIndex` (+ (`self.CurrentPatrolIndex`) (`self.PathDirection`))))
  (if (`self.IsValidMapIndex` _output_get)
    (`self.MoveToPatrolPoint`)
    (else
      (switch `/Game/Blueprints/E_PatrolPathOutcome` (`self.Patrol Path Outcome`)
        (:`NewEnumerator0`
          (set `self.CurrentPatrolIndex` 0)
          (`self.MoveToPatrolPoint`))
        (:`NewEnumerator1`
          (set `self.PathDirection` (* (`self.PathDirection`) -1))
          (set `self.CurrentPatrolIndex` (+ (`self.CurrentPatrolIndex`) (`self.PathDirection`)))
          (`self.MoveToPatrolPoint`))))))

(fn `IsValidMapIndex`
  (params (IndexToTest :type Integer))
  (returns (ReturnValue :type Boolean))
  (bind _keys (`BlueprintMapLibrary.Map_Keys` (`self.PatrolPath`)))
  (return (`KismetArrayLibrary.Array_IsValidIndex` _keys IndexToTest)))