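; Behavior tree task that plays a melee punch animation on a BP_Enemy pawn.
; If the pawn implements INT_EnemyAttack, it swaps the sprite to the potato punch flipbook, waits briefly, restores idle and finishes successfully.
; A failed cast or interface check never finishes the task.
; The MeleeAttackv3 interface message is disconnected, so the task itself triggers no attack logic.
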(event `self.ReceiveExecuteAI`
  (params (OwnerController :type "AIController Object Reference") (ControlledPawn :type "Pawn Object Reference"))
  (bind _sprite (`PaperCharacter.Sprite` (`self.Pawn`)))
  (bind _asbp_enemy (cast `/Game/Blueprints/BP_Enemy` ControlledPawn))
  (set `self.Pawn` _asbp_enemy)
  (if (`KismetSystemLibrary.DoesImplementInterface` ControlledPawn "/Game/Blueprints/INT_EnemyAttack.INT_EnemyAttack_C")
    (`PaperFlipbookComponent.SetFlipbook` _sprite "/Game/Sprites/Enemy_Potatoe/Enemy_Potatoe_Punch.Enemy_Potatoe_Punch")
    (`KismetSystemLibrary.Delay` 0.47)
    (`PaperFlipbookComponent.SetFlipbook` _sprite "/Game/Sprites/Enemy_Potatoe/Enemy_Potatoe_Idle.Enemy_Potatoe_Idle")
    (`self.FinishExecute` true)))